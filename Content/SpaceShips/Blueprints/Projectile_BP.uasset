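; Projectile Blueprint for a spaceship game that destroys rocks and awards score.
; On overlap with a Rock, it adds points to the player Ship_BP, worth more for smaller rocks via an inverse of Size.
; It then destroys itself and calls the rock's OnDeath to handle the rock's own death logic.
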(event EventBeginPlay)

(event EventTick
  (params (DeltaSeconds :type Float%20%28single-precision%29)))

(event Collision|EventActorBeginOverlap
  (params (OtherActor :type Actor%20Object%20Reference))
  (bind _asrock (Utilities|Casting|CastToRock OtherActor))
  (Utilities|FlowControl|Sequence
    (:then_0
      (bind _asship_bp (Utilities|Casting|CastToShip_BP (Game|GetPlayerCharacter 0)))
      (if (> (Variables|/Script/SpaceShips.Rock|Getsize _asrock) 0.0)
        (Variables|/Game/SpaceShips/Blueprints/Ship_BP.Ship_BP_C|SetScore _asship_bp (+ (Variables|/Game/SpaceShips/Blueprints/Ship_BP.Ship_BP_C|GetScore _asship_bp) (Math|Float|Truncate (/ 1e+02 (Variables|/Script/SpaceShips.Rock|Getsize _asrock)))))))
    (:then_1
      (Actor|DestroyActor)
      (Class|Rock|OnDeath _asrock))))

(fn ConstructionScript)