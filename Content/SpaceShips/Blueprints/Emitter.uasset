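; Emitter is a spawner actor that periodically launches Rock_BP actors once the ship game has started.
; Tick accumulates delta time and calls TriggerSpawn whenever it reaches SpawnRate, then resets the timer.
; TriggerSpawn checks IsGameStarted on the player's Ship_BP, then spawns a rock at the Arrow component's transform with randomized pitch to spread the directions.
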(event Custom|Trigger%20Spawn
  (bind _arrow (Variables|Default|GetArrow))
  (bind _returnvalue (Transformation|GetWorldRotation _arrow))
  (bind _asship_bp (Utilities|Casting|CastToShip_BP (Game|GetPlayerCharacter 0)))
  (if (Variables|/Game/SpaceShips/Blueprints/Ship_BP.Ship_BP_C|GetIsGameStarted _asship_bp)
    (Game|SpawnActorfromClass "/Game/SpaceShips/Blueprints/Rock_BP.Rock_BP_C" (Math|Transform|MakeTransform (Transformation|GetWorldLocation _arrow) (Math|Rotator|MakeRotator (.roll _returnvalue) (+ (.pitch _returnvalue) (Math|Random|RandomFloatinRange -3e+01 3e+01)) (.yaw _returnvalue)) (Transformation|GetWorldScale _arrow)) "Undefined" 0 0)))

(event EventTick
  (params (DeltaSeconds :type Float%20%28single-precision%29))
  (bind _spawnrate (Variables|Default|GetSpawnRate))
  (bind _output_get (Variables|Default|SetTime (+ DeltaSeconds (Variables|Default|GetTime))))
  (if (== (Math|Float|Min(Float) _output_get _spawnrate) _spawnrate)
    (Variables|Default|SetTime 0.0)
    (CallFunction|TriggerSpawn)))

(fn ConstructionScript)