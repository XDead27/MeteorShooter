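; Player ship for a 2D space game with rocks, wrapping its infinite map by mirroring X and Z through the origin on trigger volume overlaps.
; Rock hits call EnemyHit, then a timeline blinks the sprite and slows flight while health remains.
; Death pauses the game, inserts the score into ranked Hiscore save slots by shifting lower entries, and shows the highscore UI.
; A second timeline animates the ammo value after use.
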(event Collision|EventActorBeginOverlap
  (params (OtherActor :type Actor%20Object%20Reference))
  (bind _rootcomponent (Variables|Transformation|GetRootComponent))
  (bind _charactermovement (Variables|Character|GetCharacterMovement))
  (bind _charactermovement_2 (Variables|Character|GetCharacterMovement))
  (bind _returnvalue (Transformation|GetWorldLocation _rootcomponent))
  ;[1 1 1] Infinite Map Settings
  (Utilities|Casting|CastToTriggerVolume OtherActor
    (:then
      (Transformation|SetWorldLocation (Variables|Transformation|GetRootComponent) (* (Math|Vector|MakeVector (* (Math|Float|Sign(Float) (.x _returnvalue)) (- (Math|Float|Absolute(Float) (.x _returnvalue)) 1.0)) (.y _returnvalue) (* (- (Math|Float|Absolute(Float) (.z _returnvalue)) 1.0) (Math|Float|Sign(Float) (.z _returnvalue)))) "-1.000000,0.000000,-1.000000") false false))
    (:CastFailed
      (Utilities|Casting|CastToRock OtherActor)
      (Class|Ship|EnemyHit)
      (if (> (Variables|Default|GetHealthLeft) 0.0)
        ;[1 1 1] Hit
        (bind _healthtrack (Timeline|Health%20Timeline PlayFromStart)
          (:Update
            (if (> (Variables|Default|GetHealthLeft) 0.0)
              (Utilities|FlowControl|Sequence
                (:then_0
                  (Variables|/Script/Engine.CharacterMovementComponent|SetMaxFlySpeed _charactermovement 5e+01)
                  (Variables|/Script/Engine.CharacterMovementComponent|SetAirControl _charactermovement 0.3))
                (:then_1
                  (Development|SetHiddeninGame (Variables|Default|GetSprite) (>= _healthtrack 0.5) false)))))
          (:Finished
            (Variables|/Script/Engine.CharacterMovementComponent|SetMaxFlySpeed _charactermovement_2 3e+02)
            (Variables|/Script/Engine.CharacterMovementComponent|SetAirControl _charactermovement_2 0.6)))
        (else
          ;[1 1 1] On Dead
          (Development|SetHiddeninGame (Variables|Default|GetSprite) true false)
          (Input|DisableInput (Game|GetPlayerCharacter 0) (Game|GetPlayerController 0))
          (Game|SetGamePaused true)
          (Variables|Default|SetIsDead true)
          (bind _returnvalue_2 (SaveGame|CreateSaveGameObject "/Game/SpaceShips/Blueprints/ScoreSave.ScoreSave_C"))
          (bind _output_get (Variables|Default|SetSave%20Game%20Instance _returnvalue_2))
          (Utilities|FlowControl|Sequence
            (:then_0
              (Variables|Default|SetCont 0)
              (while (not (Variables|Default|GetTemp))
                (Variables|Default|SetCont (+ (Variables|Default|GetCont) 1))
                (bind _returnvalue_3 (SaveGame|LoadGamefromSlot (Utilities|String|Append "Hiscore" (Utilities|String|ToString(Integer) (Variables|Default|GetCont)))))
                (bind _output_get_2 (Variables|Default|SetTemp (== _returnvalue_3 0)))
                (if (not _output_get_2)
                  (bind _asscore_save (Utilities|Casting|CastToScoreSave _returnvalue_3))
                  (bind _output_get_3 (Variables|Default|SetTemp (< (Variables|/Game/SpaceShips/Blueprints/ScoreSave.ScoreSave_C|GetScore _asscore_save) (Variables|Default|GetScore))))
                  (if _output_get_3
                    (for _index (range (Variables|Default|GetCont) 10)
                      (bind _returnvalue_4 (SaveGame|LoadGamefromSlot (Utilities|String|Append "Hiscore" (Utilities|String|ToString(Integer) (- (+ (Variables|Default|GetCont) 10) _index)))))
                      (if (not (== _returnvalue_4 0))
                        (SaveGame|SaveGametoSlot _returnvalue_4 (Utilities|String|Append "Hiscore" (Utilities|String|ToString(Integer) (+ (- (+ (Variables|Default|GetCont) 10) _index) 1)))))))))
              (bind _output_get_4 (Variables|/Game/SpaceShips/Blueprints/ScoreSave.ScoreSave_C|SetSave%20Slot%20Name _output_get (Utilities|String|Append "Hiscore" (Utilities|String|ToString(Integer) (Variables|Default|GetCont))))))
            (:then_1
              (bind _output_get_5 (Variables|/Game/SpaceShips/Blueprints/ScoreSave.ScoreSave_C|SetUser%20Index _output_get 0)))
            (:then_2
              (Variables|/Game/SpaceShips/Blueprints/ScoreSave.ScoreSave_C|SetPlayer%20Name _output_get (Variables|Default|GetPlayerName)))
            (:then_3
              (Variables|/Game/SpaceShips/Blueprints/ScoreSave.ScoreSave_C|SetScore _output_get (Variables|Default|GetScore))
              (SaveGame|SaveGametoSlot _output_get _output_get_4 _output_get_5)
              (bind _returnvalue_5 (UserInterface|CreateWidget "/Game/SpaceShips/UI/Highscore_UI.Highscore_UI_C" (Game|GetPlayerController 0)))
              (UserInterface|Viewport|AddtoViewport _returnvalue_5 0))))))))

(event EventBeginPlay
  ;[1 1 1] Begin Play
  (Utilities|FlowControl|Sequence
    (:then_0
      (Variables|Default|SetAmmoTemp 1.0)
      (Variables|Default|SetScore 0))
    (:then_1
      (bind _returnvalue (UserInterface|CreateWidget "/Game/SpaceShips/UI/Player_UI.Player_UI_C" (Game|GetPlayerController 0)))
      (UserInterface|Viewport|AddtoViewport _returnvalue 0))))

(event EventAmmoUsed
  ;[1 1 1] AShooting
  (bind _ammo (Timeline|Ammo%20Graph PlayFromStart)
    (:Update
      (Variables|Default|SetAmmoTemp _ammo))
    (:Finished
      (if (>= (Variables|Default|GetAmmoLeft) 1.0)
        (Variables|Default|SetAmmoTemp 0.0)
        (else
          (Variables|Default|SetAmmoTemp 1.0))))))

(event Input|ActionEvents|InputActionPauseGame
  (params (Key :type Key%20Structure))
  (:Pressed
    (Game|SetGamePaused true)))

(fn ConstructionScript
  (Physics|SetSimulatePhysics (Variables|Default|GetSprite) false))